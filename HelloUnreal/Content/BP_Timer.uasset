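; Timer actor that runs an accelerated 24-hour clock and prints it to the screen every frame as HH:MM:SS.
; Tick adds delta time scaled a thousandfold to TotalSeconds, then derives hours, minutes and seconds with division and modulo.
; FloatTostr00 zero-pads each field by joining the tens and units digits of the floored value.
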(event `self.ReceiveTick`
  (params (DeltaSeconds :type "Float (single-precision)"))
  (bind _output_get (set `self.TotalSeconds` (+ (`self.TotalSeconds`) (* DeltaSeconds 1000.0))))
  (bind _returnvalue (/ _output_get 60.0))
  (`KismetSystemLibrary.PrintString` (`KismetStringLibrary.Concat_StrStr` (`self.floatTostr00` (mod (/ _returnvalue 60.0) 24.0)) ":" (`self.floatTostr00` (mod _returnvalue 60.0)) ":" (`self.floatTostr00` (mod _output_get 60.0))) true false))

(fn `floatTostr00`
  (params (Number :type "Float (double-precision)"))
  (returns (Str00 :type String))
  (bind _returnvalue (`KismetMathLibrary.FFloor` Number))
  (bind _returnvalue_2 (`KismetStringLibrary.Concat_StrStr` (`KismetStringLibrary.Conv_IntToString` (/ _returnvalue 10)) (`KismetStringLibrary.Conv_IntToString` (mod _returnvalue 10))))
  (if (not (`KismetStringLibrary.EqualEqual_StrStr` _returnvalue_2 (`self.Str`)))
    (return _returnvalue_2)))

(fn `UserConstructionScript`)