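; BP_HelloActor is a demo-style actor that spins while shuttling back and forth along the X axis.
; BeginPlay offsets the Sphere from the root, so the root's yaw rotation each Tick makes it orbit.
; The Sphere also spins locally at a multiple of the root's rate.
; The IsMoveRight flag reverses the root's travel at fixed X limits on either side of zero, with all motion scaled by DeltaSeconds.
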(event `self.ReceiveBeginPlay`
  ;[1 1 1] Sphere z-Rotation
  (`SceneComponent.K2_SetRelativeLocation` (`self.Sphere`) (500.0 0.0 0.0) false false))

(event `self.ReceiveTick`
  (params (DeltaSeconds :type "Float (single-precision)"))
  (bind _defaultsceneroot (`self.DefaultSceneRoot`))
  (bind _defaultsceneroot_2 (`self.DefaultSceneRoot`))
  (bind _returnvalue (* (`self.Root Speed`) DeltaSeconds))
  (bind _relativelocation_x (`KismetMathLibrary.BreakVector` (`SceneComponent.RelativeLocation` _defaultsceneroot)))
  (bind _relativelocation_x_2 (`KismetMathLibrary.BreakVector` (`SceneComponent.RelativeLocation` _defaultsceneroot_2)))
  ;[1 1 1] Root z-Rotation
  (`SceneComponent.K2_AddRelativeRotation` (`self.DefaultSceneRoot`) (`KismetMathLibrary.MakeRotator` 0.0 0.0 _returnvalue) false false)
  ;[1 1 1] Sphere z-Rotation
  (`SceneComponent.K2_AddLocalRotation` (`self.Sphere`) (`KismetMathLibrary.MakeRotator` 0.0 0.0 (* _returnvalue (`self.Sphere Speed`))) false false)
  (if (`self.IsMoveRight`)
    ;[1 1 1] 오른쪽이동
    (`SceneComponent.K2_AddRelativeLocation` _defaultsceneroot_2 (`KismetMathLibrary.MakeVector` (* DeltaSeconds (`self.Speed`))) false false)
    (set `self.IsMoveRight` (<= _relativelocation_x_2 2500.0))
    (else
      ;[1 1 1] 왼쪽이동
      (`SceneComponent.K2_AddRelativeLocation` _defaultsceneroot (`KismetMathLibrary.MakeVector` (* (* DeltaSeconds (`self.Speed`)) -1.0)) false false)
      (set `self.IsMoveRight` (<= _relativelocation_x -2500.0)))))

(fn `UserConstructionScript`)