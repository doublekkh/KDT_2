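; Solar system actor that animates the eight planets and Earth's Moon with orbital and spin motion.
; Each body pairs a Scene component, apparently an orbit pivot, with its own component for axial spin.
; Tick adds fixed per-body rotations to both around a single axis, without Delta Seconds scaling, so speeds depend on frame rate.
; BeginPlay and the construction script are empty.
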(event `self.ReceiveTick`
  (params (DeltaSeconds :type "Float (single-precision)"))
  (`SceneComponent.K2_AddRelativeRotation` (`self.SceneMercury`) (struct :`Yaw` -0.4726) false false)
  (`SceneComponent.K2_AddRelativeRotation` (`self.Mercury`) (struct :`Yaw` -0.003) false false)
  (`SceneComponent.K2_AddRelativeRotation` (`self.SceneVenus`) (struct :`Yaw` -0.3502) false false)
  (`SceneComponent.K2_AddRelativeRotation` (`self.Venus`) (struct :`Yaw` -0.0018) false false)
  (`SceneComponent.K2_AddRelativeRotation` (`self.SceneEarth`) (struct :`Yaw` -0.2978) false false)
  (`SceneComponent.K2_AddRelativeRotation` (`self.Earth`) (struct :`Yaw` -0.4651) false false)
  (`SceneComponent.K2_AddRelativeRotation` (`self.SceneMoon`) (struct :`Yaw` -0.1022) false false)
  (`SceneComponent.K2_AddRelativeRotation` (`self.Moon`) (struct :`Yaw` -0.016655) false false)
  (`SceneComponent.K2_AddRelativeRotation` (`self.SceneMars`) (struct :`Yaw` -0.2408) false false)
  (`SceneComponent.K2_AddRelativeRotation` (`self.Mars`) (struct :`Yaw` -0.2411) false false)
  (`SceneComponent.K2_AddRelativeRotation` (`self.SceneJupiter`) (struct :`Yaw` -0.1306) false false)
  (`SceneComponent.K2_AddRelativeRotation` (`self.Jupiter`) (struct :`Yaw` -12.6) false false)
  (`SceneComponent.K2_AddRelativeRotation` (`self.SceneSaturn`) (struct :`Yaw` -0.0965) false false)
  (`SceneComponent.K2_AddRelativeRotation` (`self.Saturn`) (struct :`Yaw` -9.87) false false)
  (`SceneComponent.K2_AddRelativeRotation` (`self.SceneUranus`) (struct :`Yaw` -0.0681) false false)
  (`SceneComponent.K2_AddRelativeRotation` (`self.Uranus`) (struct :`Yaw` -2.59) false false)
  (`SceneComponent.K2_AddRelativeRotation` (`self.SceneNeptune`) (struct :`Yaw` -0.0544) false false)
  (`SceneComponent.K2_AddRelativeRotation` (`self.Neptune`) (struct :`Yaw` -2.68) false false))

(fn `UserConstructionScript`)