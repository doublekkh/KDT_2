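; BP_MoveTimeLine is an actor that starts ping-pong movement of its Cube component when P is pressed, having enabled player input on BeginPlay.
; IsRight selects playing or reversing a timeline, whose value times Distance drives the Cube's relative Z.
; On finish, that scaled value sets relative X, IsRight flips and the branch repeats.
; A second, vector-driven timeline is present but never runs.
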(event `self.ReceiveBeginPlay`
  (`self.EnableInput` (`GameplayStatics.GetPlayerController` 0)))

(event `Key|P`
  (params (Key :type "Key Structure"))
  (bind _cube (`self.Cube`))
  (bind _cube_2 (`self.Cube`))
  (bind _isright (`self.IsRight`))
  (bind (_relativelocation_x _relativelocation_y _relativelocation_z) (`KismetMathLibrary.BreakVector` (`SceneComponent.RelativeLocation` _cube)))
  (bind _relativelocation_x_2 (`KismetMathLibrary.BreakVector` (`SceneComponent.RelativeLocation` _cube_2)))
  (:`Pressed`
    (if _isright :!label _label
      (bind (_direction _value) (`Timeline|타임라인` :!label _label_2)
        (:`Update`
          (`SceneComponent.K2_SetRelativeLocation` _cube_2 (`KismetMathLibrary.MakeVector` _relativelocation_x_2 0.0 (* _value (`self.Distance`))) false false))
        (:`Finished`
          (`SceneComponent.K2_SetRelativeLocation` _cube (`KismetMathLibrary.MakeVector` (* _value (`self.Distance`)) 0.0 _relativelocation_z) false false)
          (set `self.IsRight` (not _isright))
          (goto _label)))
      (else
        (goto _label_2 :!via `Reverse`)))))

(fn `UserConstructionScript`)