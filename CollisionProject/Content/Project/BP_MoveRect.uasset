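; BP_MoveRect is an actor that moves its Cube component around a square path in the relative XZ plane while playing.
; EventPlay and EventStop toggle IsPlay, and Tick adds a fixed per-frame offset, independent of delta time.
; An Int index cycles the four legs, advancing and reversing that axis's step upon exactly reaching a ±500 bound.
; Speed, MoveType and the Moveleft and MoveDown functions do not drive the active movement.
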(event `self.ReceiveBeginPlay`
  (set `self.Speed` 1000)
  (set `self.MoveType` "NewEnumerator0")
  (set `self.x_axis` 10.0)
  (set `self.z_axis` 10.0))

(event `self.ReceiveTick`
  (params (DeltaSeconds :type "Float (single-precision)"))
  (bind _cube (`self.Cube`))
  (bind _cube_2 (`self.Cube`))
  (bind (_relativelocation_x _relativelocation_y _relativelocation_z) (`KismetMathLibrary.BreakVector` (`SceneComponent.RelativeLocation` _cube)))
  (bind _relativelocation_x_2 (`KismetMathLibrary.BreakVector` (`SceneComponent.RelativeLocation` _cube_2)))
  (if (`self.IsPlay`)
    (switch `/Game/Project/EN_MoveType` (select `int` (`self.int`) :`0` "NewEnumerator0" :`1` "NewEnumerator1" :`2` "NewEnumerator2" :`3` "NewEnumerator3" :!type "/Game/Project/EN_MoveType Enum")
      (:`NewEnumerator0`
        (`SceneComponent.K2_AddRelativeLocation` _cube_2 (`KismetMathLibrary.MakeVector` (`self.x_axis`)) false false :!label _label)
        (if (not (!= _relativelocation_x_2 (* (+ (`self.int`) -1) -500.0)))
          (set `self.x_axis` (* (`self.x_axis`) -1.0))
          (set `self.int` (+ (`self.int`) 1))))
      (:`NewEnumerator1`
        (`SceneComponent.K2_AddRelativeLocation` _cube (`KismetMathLibrary.MakeVector` 0.0 0.0 (`self.z_axis`)) false false :!label _label_2)
        (if (not (!= _relativelocation_z (* (+ (`self.int`) -2) -500.0)))
          (set `self.z_axis` (* (`self.z_axis`) -1.0))
          (if (== (`self.int`) 3)
            (set `self.int` 0)
            (else
              (set `self.int` (+ (`self.int`) 1))))))
      (:`NewEnumerator2`
        (goto _label))
      (:`NewEnumerator3`
        (goto _label_2)))))

(event `/Game/ThirdPerson/Blueprints/BPI_MoveActor.EventPlay`
  (set `self.IsPlay` true))

(event `/Game/ThirdPerson/Blueprints/BPI_MoveActor.EventStop`
  (set `self.IsPlay` false))

(fn `MoveDown`
  (bind _cube (`self.Cube`))
  (bind (_relativelocation_x _relativelocation_y _relativelocation_z) (`KismetMathLibrary.BreakVector` (`SceneComponent.RelativeLocation` _cube)))
  (`SceneComponent.K2_AddRelativeLocation` _cube (`KismetMathLibrary.MakeVector` 0.0 0.0 (`self.z_axis`)) false false)
  (if (not (>= _relativelocation_z -250.0))
    (set `self.z_axis` (* (`self.z_axis`) -1.0))
    (set `self.MoveType` "NewEnumerator0")))

(fn `Moveleft`
  (bind _cube (`self.Cube`))
  (bind _relativelocation_x (`KismetMathLibrary.BreakVector` (`SceneComponent.RelativeLocation` _cube)))
  (`SceneComponent.K2_AddRelativeLocation` _cube (`KismetMathLibrary.MakeVector` (`self.x_axis`)) false false)
  (if (not (>= _relativelocation_x 0.0))
    (set `self.x_axis` (* (`self.x_axis`) -1.0))
    (set `self.MoveType` "NewEnumerator3")))

(fn `UserConstructionScript`)