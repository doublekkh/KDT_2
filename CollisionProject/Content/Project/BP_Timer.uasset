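; In-world game timer that shows elapsed play time as HH:MM:SS on a text render component.
; EventPlay and EventStop toggle counting, and Tick accumulates delta seconds while it runs.
; A helper zero-pads each field, and the text updates only when the formatted string changes.
; When that string matches EndTimeGame, input on player 0's pawn is disabled; a QuitGame call is left unconnected.
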(event `self.ReceiveTick`
  (params (DeltaSeconds :type "Float (single-precision)"))
  (bind _returnvalue (`GameplayStatics.GetPlayerController` 0))
  (if (`self.IsPlay`)
    (bind _output_get (set `self.TotalSeconds` (+ (`self.TotalSeconds`) DeltaSeconds)))
    (bind _returnvalue_2 (/ _output_get 60.0))
    (bind _returnvalue_3 (`KismetStringLibrary.Concat_StrStr` (`self.floatTostr00` (mod (/ _returnvalue_2 60.0) 24.0)) ":" (`self.floatTostr00` (mod _returnvalue_2 60.0)) ":" (`self.floatTostr00` (mod _output_get 60.0))))
    (if (not (`KismetStringLibrary.EqualEqual_StrStr` _returnvalue_3 (`self.Str`)))
      (bind _output_get_2 (set `self.Str` _returnvalue_3))
      (`TextRenderComponent.K2_SetText` (`self.TextRender`) (`KismetTextLibrary.Conv_StringToText` _output_get_2))
      (if (`KismetStringLibrary.EqualEqual_StrStr` _output_get_2 (`self.EndTimeGame`))
        (`self.DisableInput` (`Controller.K2_GetPawn` _returnvalue) _returnvalue)))))

(event `/Game/ThirdPerson/Blueprints/BPI_MoveActor.EventPlay`
  (set `self.IsPlay` true))

(event `/Game/ThirdPerson/Blueprints/BPI_MoveActor.EventStop`
  (set `self.IsPlay` false))

(fn `floatTostr00`
  (params (Number :type "Float (double-precision)"))
  (returns (Str00 :type String))
  (bind _returnvalue (`KismetMathLibrary.FFloor` Number))
  (return (`KismetStringLibrary.Concat_StrStr` (`KismetStringLibrary.Conv_IntToString` (/ _returnvalue 10)) (`KismetStringLibrary.Conv_IntToString` (mod _returnvalue 10)))))

(fn `UserConstructionScript`)