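; BP_Potal is a portal actor for the coin game that stays hidden until no coins remain in the level.
; BeginPlay hides the Potal0 component and disables its collision.
; EventCoinOverlap uses IsGetAllCoin to check whether any BP_Coin actors are left, then reveals Potal0 and restores collision if none are.
; Overlapping the actor only prints a "Potal" debug string.
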(event `self.ReceiveBeginPlay`
  (bind _potal_0 (`self.Potal_0`))
  (`SceneComponent.SetHiddenInGame` _potal_0 true false)
  (`PrimitiveComponent.SetCollisionEnabled` _potal_0 "NoCollision"))

(event `self.ReceiveActorBeginOverlap`
  (params (OtherActor :type "Actor Object Reference"))
  (`KismetSystemLibrary.PrintString` "Potal" true false (struct :`R` 1.0 :`B` 0.05578 :`A` 1.0)))

(fn `EventCoinOverlap`
  (bind _potal_0 (`self.Potal_0`))
  (bind _is_get_all (`self.IsGetAllCoin`))
  (if _is_get_all
    (`SceneComponent.SetHiddenInGame` _potal_0 false false)
    (`PrimitiveComponent.SetCollisionEnabled` _potal_0 "QueryAndPhysics")))

(fn `IsGetAllCoin`
  (returns (`Is Get All` :type Boolean))
  (bind _outactors (`GameplayStatics.GetAllActorsOfClass` "/Game/CoinGame/BP_Coin.BP_Coin_C"))
  (if (`KismetArrayLibrary.Array_IsEmpty` _outactors)
    (return true)))

(fn `UserConstructionScript`)