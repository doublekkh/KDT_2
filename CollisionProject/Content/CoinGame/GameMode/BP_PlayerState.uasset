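; Player state for the coin game that records pickups and shows them on the HUD.
; AddCoin increments its own Coin count and copies it to the BP_HUD widget of player 0.
; The booster, jump and double jump functions increment counters stored directly on that widget, so those totals live only in the UI.
; An unconnected, unfinished branch looks up hidden BP_Potal actors at a coin threshold but never runs.
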(fn `Add Double Jump Item`
  (bind _asbp_hud (cast `/Game/CoinGame/GameMode/BP_HUD` (`PlayerController.GetHUD` (`self.GetPlayerController`))))
  (bind _hudwidget (`/Game/CoinGame/GameMode/BP_HUD.HudWidget` _asbp_hud))
  (set `/Game/CoinGame/HudWidget.DoubleJump` (+ (`/Game/CoinGame/HudWidget.DoubleJump` _hudwidget) 1) _hudwidget))

(fn `AddBoosterItem`
  (bind _asbp_hud (cast `/Game/CoinGame/GameMode/BP_HUD` (`PlayerController.GetHUD` (`self.GetPlayerController`))))
  (bind _hudwidget (`/Game/CoinGame/GameMode/BP_HUD.HudWidget` _asbp_hud))
  (set `/Game/CoinGame/HudWidget.Booster` (+ (`/Game/CoinGame/HudWidget.Booster` _hudwidget) 1) _hudwidget))

(fn `AddCoin`
  (bind _output_get (set `self.Coin` (+ (`self.Coin`) 1)))
  (bind _asbp_hud (cast `/Game/CoinGame/GameMode/BP_HUD` (`PlayerController.GetHUD` (`GameplayStatics.GetPlayerController` 0))))
  (set `/Game/CoinGame/HudWidget.Coin` _output_get (`/Game/CoinGame/GameMode/BP_HUD.HudWidget` _asbp_hud)))

(fn `AddJumpItem`
  (bind _asbp_hud (cast `/Game/CoinGame/GameMode/BP_HUD` (`PlayerController.GetHUD` (`self.GetPlayerController`))))
  (bind _hudwidget (`/Game/CoinGame/GameMode/BP_HUD.HudWidget` _asbp_hud))
  (set `/Game/CoinGame/HudWidget.Jump` (+ (`/Game/CoinGame/HudWidget.Jump` _hudwidget) 1) _hudwidget))

(fn `UserConstructionScript`)