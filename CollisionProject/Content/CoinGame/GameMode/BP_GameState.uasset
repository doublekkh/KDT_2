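; Game state for the coin game that runs the match countdown and signals its end.
; Each Tick, SetTimer reduces GameTimer and writes it as MM:SS to the HUD widget's Time, using FtoStr for two-digit padding.
; When the returned text equals "00:00", it calls GameSetMessage on actors tagged CoinGame and disables its own tick inside that loop.
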(event `self.ReceiveTick`
  (params (DeltaSeconds :type "Float (single-precision)"))
  (bind _newtime (`self.SetTimer` DeltaSeconds))
  ;[1 1 1] Game Set
  (if (`KismetStringLibrary.EqualEqual_StrStr` _newtime "00:00")
    (bind _outactors (`GameplayStatics.GetAllActorsWithTag` "CoinGame"))
    (for _array_element _outactors
      (message `/Game/CoinGame/BPI_GameSet.GameSet` _array_element)
      (`self.SetActorTickEnabled` false))))

(fn `FtoStr`
  (params (Number :type "Float (double-precision)"))
  (returns (Str00 :type String))
  (bind _returnvalue (`KismetMathLibrary.FFloor` Number))
  (bind _returnvalue_2 (`KismetStringLibrary.Concat_StrStr` (`KismetStringLibrary.Conv_IntToString` (/ _returnvalue 10)) (`KismetStringLibrary.Conv_IntToString` (mod _returnvalue 10))))
  (if (not (`KismetStringLibrary.EqualEqual_StrStr` _returnvalue_2 (`self.Str`)))
    (return _returnvalue_2)))

(fn `SetTimer`
  (params (DeltaSec :type "Float (double-precision)"))
  (returns (NewTime :type String))
  (bind _output_get (set `self.GameTimer` (- (`self.GameTimer`) DeltaSec)))
  (bind _asbp_hud (cast `/Game/CoinGame/GameMode/BP_HUD` (`PlayerController.GetHUD` (`GameplayStatics.GetPlayerController` 0))))
  (bind _output_get_2 (set `/Game/CoinGame/HudWidget.Time` (`KismetStringLibrary.Concat_StrStr` (`self.FtoStr` (/ _output_get 60.0)) ":" (`self.FtoStr` (mod _output_get 60.0))) (`/Game/CoinGame/GameMode/BP_HUD.HudWidget` _asbp_hud)))
  (return _output_get_2))

(fn `UserConstructionScript`)