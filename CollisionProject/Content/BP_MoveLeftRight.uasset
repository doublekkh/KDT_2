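; BP_MoveLeftRight is an actor that spins a sphere in orbit around its root, despite its name.
; BeginPlay offsets the sphere along X, then Tick yaws the root and spins the sphere locally at a multiple of that speed, scaled by delta time.
; EventPlay and EventStop toggle the IsPlay flag that gates this motion.
; An unconnected left/right ping-pong movement along X remains in the graph but never runs.
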(event `self.ReceiveBeginPlay`
  ;[1 1 1] Sphere z-Rotation
  (`SceneComponent.K2_SetRelativeLocation` (`self.Sphere`) (500.0 0.0 0.0) false false))

(event `self.ReceiveTick`
  (params (DeltaSeconds :type "Float (single-precision)"))
  (bind _returnvalue (* (`self.Root Speed`) DeltaSeconds))
  (if (`self.IsPlay`)
    ;[1 1 1] Root z-Rotation
    (`SceneComponent.K2_AddRelativeRotation` (`self.DefaultSceneRoot`) (`KismetMathLibrary.MakeRotator` 0.0 0.0 _returnvalue) false false)
    ;[1 1 1] Sphere z-Rotation
    (`SceneComponent.K2_AddLocalRotation` (`self.Sphere`) (`KismetMathLibrary.MakeRotator` 0.0 0.0 (* _returnvalue (`self.Sphere Speed`))) false false)))

(event `/Game/ThirdPerson/Blueprints/BPI_MoveActor.EventPlay`
  (set `self.IsPlay` true))

(event `/Game/ThirdPerson/Blueprints/BPI_MoveActor.EventStop`
  (set `self.IsPlay` false))

(fn `UserConstructionScript`)